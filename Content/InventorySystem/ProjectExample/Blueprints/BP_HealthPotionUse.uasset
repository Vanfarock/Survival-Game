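; Health potion use item that temporarily boosts the player character's health regeneration.
; On use, it casts the player pawn, saves HealthRecover and sets it to the larger of the boosted value and HealthRegenCap, so the cap acts as a floor.
; A ten-second named timer calls ResetHealthRegen to restore the saved value through the Player reference, which IncreaseHealthRegen appears to set to None.
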(event `self.DoUseItem (DO OVERRIDE)`
  (bind _asch_inventory_system_character (cast `/Game/InventorySystem/ProjectExample/Blueprints/CH_InventorySystemCharacter` (`GameplayStatics.GetPlayerPawn` 0)))
  (`self.IncreaseHealthRegen` _asch_inventory_system_character)
  (`KismetSystemLibrary.K2_SetTimer` null "ResetHealthRegen" 10.0))

(fn `IncreaseHealthRegen`
  (params (Player :type "/Game/InventorySystem/ProjectExample/Blueprints/CH_InventorySystemCharacter Object Reference"))
  (bind _healthrecover (`/Game/InventorySystem/ProjectExample/Blueprints/CH_InventorySystemCharacter.HealthRecover` Player))
  (set `self.Player` null)
  (set `self.OriginalHealthRegen` _healthrecover)
  (set `/Game/InventorySystem/ProjectExample/Blueprints/CH_InventorySystemCharacter.HealthRecover` (`KismetMathLibrary.FMax` (+ _healthrecover (`self.HealthRegen`)) (`self.HealthRegenCap`)) Player))

(fn `ResetHealthRegen`
  (set `/Game/InventorySystem/ProjectExample/Blueprints/CH_InventorySystemCharacter.HealthRecover` (`self.OriginalHealthRegen`) (`self.Player`)))

(fn `UserConstructionScript`)