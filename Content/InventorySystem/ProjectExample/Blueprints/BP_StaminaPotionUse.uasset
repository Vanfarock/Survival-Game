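; Stamina potion use action for the inventory example, meant to temporarily boost the player character's stamina recovery rate.
; On use, it stores the original rate and sets the higher of the boosted rate or StaminaRegenCap, so the cap acts as a floor.
; A ten-second timer targets DecreaseStaminaRegen, which is absent here.
; The restore function is named ResetHealthRegen, takes a Player parameter and is never called in this Blueprint.
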(event `self.DoUseItem (DO OVERRIDE)`
  (bind _asch_inventory_system_character (cast `/Game/InventorySystem/ProjectExample/Blueprints/CH_InventorySystemCharacter` (`GameplayStatics.GetPlayerPawn` 0)))
  (`self.IncreaseStaminaRegen` _asch_inventory_system_character)
  (`KismetSystemLibrary.K2_SetTimer` null "DecreaseStaminaRegen" 10.0))

(fn `IncreaseStaminaRegen`
  (params (Player :type "/Game/InventorySystem/ProjectExample/Blueprints/CH_InventorySystemCharacter Object Reference"))
  (bind _staminarecoveryrate (`/Game/InventorySystem/ProjectExample/Blueprints/CH_InventorySystemCharacter.StaminaRecoveryRate` Player))
  (set `self.Player` Player)
  (set `self.OriginalStaminaRegen` _staminarecoveryrate)
  (set `/Game/InventorySystem/ProjectExample/Blueprints/CH_InventorySystemCharacter.StaminaRecoveryRate` (`KismetMathLibrary.FMax` (+ _staminarecoveryrate (`self.StaminaRegen`)) (`self.StaminaRegenCap`)) Player))

(fn `ResetHealthRegen`
  (params (Player :type "/Game/InventorySystem/ProjectExample/Blueprints/CH_InventorySystemCharacter Object Reference"))
  (set `/Game/InventorySystem/ProjectExample/Blueprints/CH_InventorySystemCharacter.StaminaRecoveryRate` (`self.OriginalStaminaRegen`) Player))

(fn `UserConstructionScript`)